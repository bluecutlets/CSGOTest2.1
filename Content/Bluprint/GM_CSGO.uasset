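; CS:GO-style game mode that tracks connected players and handles their team spawn requests.
; On each PostLogin it records the controller and refreshes its lists of Counter-Terrorist and Terrorist spawn point actors.
; A spawn request picks a random point from each list, selects the transform matching the requested team, and passes it to the player's SpawnActor.
; GameCSGOref returns the game mode itself as a reference.
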(event `self.K2_PostLogin`
  (params (NewPlayer :type "PlayerController Object Reference"))
  (`KismetArrayLibrary.Array_AddUnique` (`self.ConectedPlayer`) NewPlayer)
  (bind _outactors (`GameplayStatics.GetAllActorsOfClass` "/Game/Bluprint/Player/SpawnPoints/BP_Spawn_ContrTerrorist.BP_Spawn_ContrTerrorist_C"))
  (set `self.ContrTerrorist` _outactors)
  (bind _outactors_2 (`GameplayStatics.GetAllActorsOfClass` "/Game/Bluprint/Player/SpawnPoints/BP_Spawn_Terrorist.BP_Spawn_Terrorist_C"))
  (set `self.Terrorist` _outactors_2))

(event `RequstSpawnPlayer`
  (params (Player :type "/Game/Bluprint/PC_CSGO Object Reference") (Team :type "Actor Class Reference"))
  (`/Game/Bluprint/PC_CSGO.SpawnActor` Player Team (`KismetMathLibrary.SelectTransform` (`self.GetTransform` (`KismetArrayLibrary.Array_Random` (`self.ContrTerrorist`))) (`self.GetTransform` (`KismetArrayLibrary.Array_Random` (`self.Terrorist`))) (== Team "/Game/Bluprint/Player/BP_ContrTerorist.BP_ContrTerorist_C"))))

(fn `GameCSGOref`
  (returns (Gamemode :type "/Game/Bluprint/GM_CSGO Object Reference"))
  (return self))

(fn `UserConstructionScript`)