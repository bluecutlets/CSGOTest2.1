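; Player controller for a CS:GO-style game that handles team selection, pawn spawning and UI switching.
; On BeginPlay it views a level CameraActor and shows the team menu; SelectTeam forwards the choice through an SRV_ event to the game mode.
; SpawnActor spawns and possesses the team's pawn, then a CI_ event swaps to the main widget and game-only input.
; Widgets are created lazily, cached and toggled by enum.
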(event `CI_SpawnPlayer`
  (`self.ShowHiddenWidget` "NewEnumerator0")
  (`self.ShowHiddenWidget` "NewEnumerator1" true)
  (`WidgetBlueprintLibrary.SetInputMode_GameOnly` self)
  (set `self.bShowMouseCursor` false))

(event `self.ReceiveBeginPlay`
  (`self.ShowHiddenWidget` "NewEnumerator0" true)
  (bind _gamemode (message `/Game/Bluprint/Player/interface/INT_Gamemode.GameCSGOref` (`GameplayStatics.GetGameMode`)))
  (set `self.Gamemode` _gamemode)
  (bind _returnvalue (`GameplayStatics.GetActorOfClass` "/Script/Engine.CameraActor"))
  (`self.SetViewTargetWithBlend` _returnvalue)
  (`WidgetBlueprintLibrary.SetInputMode_UIOnlyEx` self null)
  (set `self.bShowMouseCursor` true))

(event `ShowHiddenWidget`
  (params (Widget :type "/Game/Bluprint/Player/Enum/E_GameWIdget Enum" :default "NewEnumerator0") (Show :type Boolean))
  (`self.CI_ShowWidget` Widget Show))

(event `CI_ShowWidget`
  (params (Widget :type "/Game/Bluprint/Player/Enum/E_GameWIdget Enum" :default "NewEnumerator0") (Show :type Boolean))
  (if Show
    (`self.F_ShowWidget` Widget)
    (else
      (`self.F_HiddenWidget` Widget))))

(event `SpawnActor`
  (params (Team :type "Actor Class Reference") (SpawnTransform :type "Transform Structure"))
  (bind _returnvalue (`|SpawnActorFromClass` Team SpawnTransform "AdjustIfPossibleButAlwaysSpawn" "MultiplyWithRoot" null null))
  (bind _output_get (set `self.PlayerPawn` _returnvalue))
  (bind _player (message `/Game/Bluprint/Player/interface/INT_PlayerRef.GetpalyerRef` _output_get))
  (`self.Possess` _player)
  (`self.CI_SpawnPlayer`))

(event `SelectTeam`
  (params (Team :type "Actor Class Reference"))
  (`self.SRV_SelectTeam` Team))

(event `SRV_SelectTeam`
  (params (Team :type "Actor Class Reference"))
  (`/Game/Bluprint/GM_CSGO.RequstSpawnPlayer` (`self.Gamemode`) self Team))

(fn `F_HiddenWidget`
  (params (Widget :type "/Game/Bluprint/Player/Enum/E_GameWIdget Enum" :default "NewEnumerator0"))
  (switch `/Game/Bluprint/Player/Enum/E_GameWIdget` Widget
    (:`NewEnumerator0`
      (bind _teamselection (`self.TeamSelection`)
        (:`then`
          (`Widget.RemoveFromParent` _teamselection))
        (:`else`)))
    (:`NewEnumerator1`
      (bind _wb_main1 (`self.WB_Main1`)
        (:`then`
          (`Widget.RemoveFromParent` _wb_main1))
        (:`else`)))))

(fn `F_ShowWidget`
  (params (Widget :type "/Game/Bluprint/Player/Enum/E_GameWIdget Enum" :default "NewEnumerator0"))
  (switch `/Game/Bluprint/Player/Enum/E_GameWIdget` Widget
    (:`NewEnumerator0`
      (`self.TeamSelection`
        (:`then`
          _)
        (:`else`
          (bind _returnvalue (`|CreateWidget` "/Game/UI/WB_ChoiceSpawn.WB_ChoiceSpawn_C"))
          (bind _output_get (set `self.TeamSelection` _returnvalue))))
      (`UserWidget.AddToViewport` _output_get 0))
    (:`NewEnumerator1`
      (`self.WB_Main1`
        (:`then`
          _)
        (:`else`
          (bind _returnvalue_2 (`|CreateWidget` "/Game/UI/WB_Main.WB_Main_C"))
          (bind _output_get_2 (set `self.WB_Main1` _returnvalue_2))))
      (`UserWidget.AddToViewport` _output_get_2 0))))

(fn `Get Controller Player ref`
  (returns (PlayerController :type "/Game/Bluprint/PC_CSGO Object Reference"))
  (return self))

(fn `UserConstructionScript`)