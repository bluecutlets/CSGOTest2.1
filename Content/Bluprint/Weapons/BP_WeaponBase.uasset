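; Base weapon actor for a networked game, acting as a physics-simulated pickup that players can loot.
; On BeginPlay it enables physics and sets current and extra ammo from its weapon info through a server-named init event.
; When a tagged player overlaps its sphere, the authority checks that player's inventory for the same weapon type.
; It registers itself as an overlapped item only if none matches, using a temporary loot flag on the player.
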(event `SRV_InilizeWeapon`
  (bind ((`Maxbullet_29_F80D887643CCD82F189C44B802D30EA5` _maxbullet) (`MaxExtrabullet_31_C2FCCDC74E43A60ADC3C43ABD270199E` _maxextrabullet)) (break `/Game/Bluprint/Player/Struct/ST_Weapon` (`/Game/Bluprint/Player/Struct/F_Weapon.F_WeaponInfo` (`self.Name`))))
  (set `self.Current Ammo` _maxbullet)
  (set `self.ExraAmmo` _maxextrabullet))

(event `self.ReceiveBeginPlay`
  (`PrimitiveComponent.SetSimulatePhysics` (`self.Weapon`) true)
  (`self.SRV_InilizeWeapon`))

(event `self.Sphere.OnComponentBeginOverlap`
  (params (OverlappedComponent :type "PrimitiveComponent Object Reference") (OtherActor :type "Actor Object Reference") (OtherComp :type "PrimitiveComponent Object Reference") (OtherBodyIndex :type Integer) (bFromSweep :type Boolean) (SweepResult :type "HitResult Structure (by ref)"))
  (if (`self.ActorHasTag` OtherActor "player")
    (`/Engine/EditorBlueprintResources/ActorMacros.Switch Has Authority`
      (:`Authority`
        (bind _player (message `/Game/Bluprint/Player/interface/INT_PlayerRef.GetpalyerRef` OtherActor))
        (for _array_element (`/Game/Bluprint/Player/BP_PlayerBase.WeaponInventori` _player)
          (if (`|EnumEquality` (`.Type_4_43B433C848D99C570C16E59FFDBC5672` (break `/Game/Bluprint/Player/Struct/ST_Weapon` (`/Game/Bluprint/Player/Struct/F_Weapon.F_WeaponInfo` (`/Game/Bluprint/Weapons/BP_WeaponBase.Name` _array_element)))) (`.Type_4_43B433C848D99C570C16E59FFDBC5672` (break `/Game/Bluprint/Player/Struct/ST_Weapon` (`/Game/Bluprint/Player/Struct/F_Weapon.F_WeaponInfo` (`self.Name`)))))
            (set `/Game/Bluprint/Player/BP_PlayerBase.YoucanLootWeapon` false _player)
            (break)))
        (if (`/Game/Bluprint/Player/BP_PlayerBase.YoucanLootWeapon` _player)
          (`/Game/Bluprint/Player/BP_PlayerBase.AddOverlappeditem` _player self)
          (else
            (set `/Game/Bluprint/Player/BP_PlayerBase.YoucanLootWeapon` true _player)))))))

(fn `UserConstructionScript`)