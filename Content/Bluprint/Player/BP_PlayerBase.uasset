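; Networked base player character with a first-person body (head bone hidden), handling Enhanced Input movement, crouch, walk, footsteps and rifle use.
; Server RPCs run weapon looting from overlaps, dropping and looped firing, with multicasts playing sounds, muzzle flash and reload montage.
; OnRep functions attach or physically drop weapons.
; Shots trace from camera points sent by the owner, but player hits only print a debug string.
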(event `self.ReceiveBeginPlay`
  (`KismetSystemLibrary.Delay` 0.01)
  (bind _playercontroller (message `/Game/Bluprint/Player/interface/INT_PlayerController.Get Controller Player ref` (`self.GetController`)))
  (`/Engine/EditorBlueprintResources/StandardMacros.IsValid` _playercontroller
    (:`Is Valid`
      (bind _returnvalue (pcsubsystem `EnhancedInputLocalPlayerSubsystem` _playercontroller))
      (`/Engine/EditorBlueprintResources/StandardMacros.IsValid` _returnvalue
        (:`Is Valid`
          (`EnhancedInputSubsystemInterface.AddMappingContext` _returnvalue "/Game/Bluprint/Player/Input/INC_Defult.INC_Defult" 0 (struct))
          (`SkinnedMeshComponent.HideBoneByName` (`self.Mesh`) "head" "PBO_None"))))))

(event `EnhancedInput|/Game/Bluprint/Player/Input/IN_Movement`
  (params (ActionValue :type "Vector2D Structure") (ElapsedSeconds :type "Float (double-precision)") (TriggeredSeconds :type "Float (double-precision)") (InputAction :type "InputAction Object Reference" :default "/Game/Bluprint/Player/Input/IN_Movement.IN_Movement"))
  (bind (_x _y) (`KismetMathLibrary.BreakVector3f` (`self.GetVelocity`)))
  ;[0.001347 0.0101 0.1094] Movement
  (:`Triggered`
    (`self.AddMovementInput` (`self.GetActorForwardVector`) ActionValue_X)
    (`self.AddMovementInput` (`self.GetActorRightVector`) ActionValue_Y)
    (if (and (or (> _x 250.0) (< _x -250.0) (> _y 250.0) (< _y -250.0)) (`self.f_jump`) (not (`self.bCrouch`)) (not (`self.bWalk`)))
      (if (not (`self.PlayingFootStaps`))
        (set `self.PlayingFootStaps` true)
        (`self.SRV_FootstepsSFX`)
        (bind _returnvalue (`KismetSystemLibrary.K2_SetTimerDelegate` (delegate `Foot_steps_SFX`) 0.42 true))
        (set `self.Footsteps` _returnvalue))
      (else
        (if (`KismetSystemLibrary.K2_IsValidTimerHandle` (`self.Footsteps`)) :!label _label
          (`KismetSystemLibrary.K2_ClearAndInvalidateTimerHandle` (`self.Footsteps`))
          (set `self.PlayingFootStaps` false)))))
  (:`Completed`
    (goto _label)))

(event `Foot_steps_SFX`
  ;[0.001347 0.0101 0.1094] Movement
  (`self.SRV_FootstepsSFX`))

(event `SRV_FootstepsSFX`
  ;[0.001347 0.0101 0.1094] Movement
  (`self.MC_Footsteps`))

(event `MC_Footsteps`
  ;[0.001347 0.0101 0.1094] Movement
  (`GameplayStatics.PlaySoundAtLocation` "/Game/Audio/SFX/S_FootSteps.S_FootSteps" (`self.K2_GetActorLocation`) (struct) 1.0 1.0 0.0 null null null null))

(event `EnhancedInput|/Game/Bluprint/Player/Input/IA_Look`
  (params (ActionValue :type "Vector2D Structure") (ElapsedSeconds :type "Float (double-precision)") (TriggeredSeconds :type "Float (double-precision)") (InputAction :type "InputAction Object Reference" :default "/Game/Bluprint/Player/Input/IA_Look.IA_Look"))
  ;[0.001347 0.0101 0.1094] movement Camera
  (:`Triggered`
    (`self.AddControllerYawInput` ActionValue_X)
    (`self.AddControllerPitchInput` ActionValue_Y)))

(event `EnhancedInput|/Game/Bluprint/Player/Input/IA_Crouch`
  (params (ActionValue :type Boolean) (ElapsedSeconds :type "Float (double-precision)") (TriggeredSeconds :type "Float (double-precision)") (InputAction :type "InputAction Object Reference" :default "/Game/Bluprint/Player/Input/IA_Crouch.IA_Crouch"))
  ;[0.001347 0.0101 0.1094] Controller Movement
  (:`Triggered`
    (if (`self.f_jump`) :!label _label_2
      (if ActionValue
        (`self.F_Crouch` true)
        (else
          (`self.F_Crouch` false)))
      (else
        (`KismetSystemLibrary.Delay` 0.05)
        (goto _label_2)))))

(event `SRV_WAlk`
  (params (state :type Boolean))
  ;[0.001347 0.0101 0.1094] Controller Movement
  (`self.F_Walk` state))

(event `CI_UPUserUI`
  (params (Texture :type "Texture2D Object Reference"))
  ;[0.001347 0.0101 0.1094] UI Weapon
  (bind _playercontroller (message `/Game/Bluprint/Player/interface/INT_PlayerController.Get Controller Player ref` (`self.GetController`)))
  (`/Game/UI/WB_Main.UpdateUIInvetori` (`/Game/Bluprint/PC_CSGO.WB_Main1` _playercontroller) Texture))

(event `SRV_Crouch`
  (params (bCrouch :type Boolean))
  ;[0.001347 0.0101 0.1094] Controller Movement
  (`self.F_Crouch` bCrouch))

(event `EnhancedInput|/Game/Bluprint/Player/Input/IA_Jump`
  (params (ActionValue :type Boolean) (ElapsedSeconds :type "Float (double-precision)") (TriggeredSeconds :type "Float (double-precision)") (InputAction :type "InputAction Object Reference" :default "/Game/Bluprint/Player/Input/IA_Jump.IA_Jump"))
  ;[0.001347 0.0101 0.1094] Controller Movement
  (:`Triggered`
    (if (`self.f_jump`)
      (`self.Jump`))))

(event `EnhancedInput|/Game/Bluprint/Player/Input/IA_WALK`
  (params (ActionValue :type Boolean) (ElapsedSeconds :type "Float (double-precision)") (TriggeredSeconds :type "Float (double-precision)") (InputAction :type "InputAction Object Reference" :default "/Game/Bluprint/Player/Input/IA_WALK.IA_WALK"))
  ;[0.001347 0.0101 0.1094] Controller Movement
  (:`Triggered`
    (if ActionValue
      (`self.F_Walk` true)
      (else
        (`self.F_Walk` false)))))

(event `LootWeapon`
  ;[0.001347 0.0101 0.1094] Loot Weapon
  (`self.SRV_LootWeapon`))

(event `SRV_LootWeapon`
  (bind _weaponinventori (`self.WeaponInventori`))
  (bind _overlapweapons (`self.overlapWeapons`))
  (bind _output (`|GetArrayItem` _overlapweapons))
  (bind ((`Type_4_43B433C848D99C570C16E59FFDBC5672` _type) (`texture_14_1D9C6DCC4437B1C3C99FD3B6AD8D0F04` _texture)) (break `/Game/Bluprint/Player/Struct/ST_Weapon` (`/Game/Bluprint/Player/Struct/F_Weapon.F_WeaponInfo` (`/Game/Bluprint/Weapons/BP_WeaponBase.Name` (`self.Weapon`)))))
  ;[0.001347 0.0101 0.1094] Loot Weapon
  (if (`KismetArrayLibrary.Array_IsNotEmpty` _overlapweapons)
    (`KismetArrayLibrary.Array_Set` _weaponinventori (`KismetArrayLibrary.Array_Length` _weaponinventori) _output true)
    (bind _output_get (set `self.Weapon` _output))
    (set `self.EqipedWeapon` _output_get)
    (if (`|EnumEquality` (`self.EqiupWeapon`) "NewEnumerator0")
      (`KismetSystemLibrary.Delay` 0.1)
      (`self.SetEquipedWeapon` _type)
      (`self.SetsEquipWeapon` true)
      (`self.CI_UPUserUI` _texture)
      (`KismetArrayLibrary.Array_RemoveItem` (`self.overlapWeapons`) _output)
      (`self.CheckoverlapWeapon`))
    (else
      (`self.CanLootWeaponsAgain`)
      (`KismetSystemLibrary.Delay` 0.1)
      (set `self.Weapon` null))))

(event `AddOverlappeditem`
  (params (Weapon :type "/Game/Bluprint/Weapons/BP_WeaponBase Object Reference"))
  ;[0.001347 0.0101 0.1094] Loot Weapon
  (`self.SRV_AddOverlappeditem` Weapon))

(event `CheckoverlapWeapon`
  ;[0.001347 0.0101 0.1094] Loot Weapon
  (`self.LootWeapon` :!label _label_3))

(event `SRV_AddOverlappeditem`
  (params (Weapon :type "/Game/Bluprint/Weapons/BP_WeaponBase Object Reference"))
  (bind _overlapweapons (`self.overlapWeapons`))
  ;[0.001347 0.0101 0.1094] Loot Weapon
  (`KismetArrayLibrary.Array_Set` _overlapweapons (`KismetArrayLibrary.Array_Length` _overlapweapons) Weapon true)
  (`/Engine/EditorBlueprintResources/StandardMacros.DoOnce` false :!label _label_4
    (:`Completed`
      (goto _label_3))))

(event `CanLootWeaponsAgain`
  ;[0.001347 0.0101 0.1094] Loot Weapon
  (goto _label_4 :!via `Reset`))

(event `SetEquipedWeapon`
  (params (EqiupWeapon :type "/Game/Bluprint/Player/Enum/Weapon_Type Enum" :default "NewEnumerator0"))
  ;[0.001347 0.0101 0.1094] Equp Weapon
  (`self.SRV_SetEquipedWeapon` EqiupWeapon))

(event `EnhancedInput|/Game/Bluprint/Player/Input/IA_Drop_Weapon`
  (params (ActionValue :type Boolean) (ElapsedSeconds :type "Float (double-precision)") (TriggeredSeconds :type "Float (double-precision)") (InputAction :type "InputAction Object Reference" :default "/Game/Bluprint/Player/Input/IA_Drop_Weapon.IA_Drop_Weapon"))
  ;[0.001347 0.0101 0.1094] Drop Weapon
  (:`Triggered`
    (if (`|EnumInequality` (`self.EqiupWeapon`) "NewEnumerator0")
      (`self.SRV_DropWeapon`))))

(event `SRV_SetEquipedWeapon`
  (params (EqiupWeapon :type "/Game/Bluprint/Player/Enum/Weapon_Type Enum" :default "NewEnumerator0"))
  ;[0.001347 0.0101 0.1094] Equp Weapon
  (set `self.EqiupWeapon` EqiupWeapon))

(event `EnhancedInput|/Game/Bluprint/Player/Input/IA_reload`
  (params (ActionValue :type Boolean) (ElapsedSeconds :type "Float (double-precision)") (TriggeredSeconds :type "Float (double-precision)") (InputAction :type "InputAction Object Reference" :default "/Game/Bluprint/Player/Input/IA_reload.IA_reload"))
  ;[0.001347 0.0101 0.1094] Equp Weapon
  (:`Triggered`
    (set `self.brealod` true)
    (`self.MC_EquipWeapon` "NewEnumerator1")))

(event `SRV_DropWeapon`
  ;[0.001347 0.0101 0.1094] Drop Weapon
  (for _array_element (`self.WeaponInventori`)
    (if (`|EnumEquality` (`self.EqiupWeapon`) (`.Type_4_43B433C848D99C570C16E59FFDBC5672` (break `/Game/Bluprint/Player/Struct/ST_Weapon` (`/Game/Bluprint/Player/Struct/F_Weapon.F_WeaponInfo` (`/Game/Bluprint/Weapons/BP_WeaponBase.Name` _array_element)))))
      (set `self.dropweapon` _array_element)
      (`KismetArrayLibrary.Array_RemoveItem` (`self.WeaponInventori`) _array_element)
      (`self.CI_UPUserUI` null)
      (set `self.EqiupWeapon` "NewEnumerator0")
      (break)))
  (`KismetSystemLibrary.Delay` 0.1)
  (set `self.dropweapon` null))

(event `MC_EquipWeapon`
  (params (`Weapon Type ` :type "/Game/Bluprint/Player/Enum/Weapon_Type Enum" :default "NewEnumerator0"))
  ;[0.001347 0.0101 0.1094] Equp Weapon
  (`|PlayMontage` (`self.Mesh`) (select `/Game/Bluprint/Player/Enum/Weapon_Type` `Weapon Type ` :`NewEnumerator1` "/Game/Assets/Animetions/A_ReloadRifle.A_ReloadRifle" :!type "AnimMontage Object Reference")
    (:`OnCompleted`
      (set `self.brealod` false)
      (`self.SetsEquipWeapon` false))))

(event `EnhancedInput|/Game/Bluprint/Player/Input/IA_ire`
  (params (ActionValue :type Boolean) (ElapsedSeconds :type "Float (double-precision)") (TriggeredSeconds :type "Float (double-precision)") (InputAction :type "InputAction Object Reference" :default "/Game/Bluprint/Player/Input/IA_ire.IA_ire"))
  (bind (_returnvalue _returnvalue2) (`self.LineTraseShoot`))
  (:`Triggered`
    (if (and (not (`self.bIsEqipWeapon`)) (`|EnumInequality` (`self.EqiupWeapon`) "NewEnumerator0") (not (`self.brealod`)))
      (bind _eqipedweapon (`self.EqipedWeapon`)
        (:`then`
          (`self.SRV_Fire` _eqipedweapon true _returnvalue _returnvalue2))
        (:`else`))))
  (:`Completed`
    (`self.SRV_Fire` (`self.EqipedWeapon`))))

(event `SRV_Fire`
  (params (Weapon :type "/Game/Bluprint/Weapons/BP_WeaponBase Object Reference") (bShootWeapon :type Boolean) (Start :type "Vector Structure") (End :type "Vector Structure"))
  (bind _shootweaponend (`self.ShootWeaponEnd`))
  (if bShootWeapon
    (`/Engine/EditorBlueprintResources/StandardMacros.DoOnce` false :!label _label_5
      (:`Completed`
        (`self.FirstShoot`)
        (bind _returnvalue (`KismetSystemLibrary.K2_SetTimerDelegate` (delegate `ShootWeaponLoop`) 0.1 true))
        (set `self.ShootWeaponEnd` _returnvalue)))
    (elif (`KismetSystemLibrary.K2_IsValidTimerHandle` _shootweaponend)
      (`KismetSystemLibrary.K2_ClearAndInvalidateTimerHandle` _shootweaponend)
      (`self.CanShootAgen`))))

(event `CanShootAgen`
  (goto _label_5 :!via `Reset`))

(event `FirstShoot`
  (bind ((`MuzzleFlash_23_8E9B851C4F7DE530FB45269B50A313D5` _muzzleflash) (`SoundSFX_26_EFDA4CFD4EAFADF750298D9A49ABED6E` _soundsfx)) (break `/Game/Bluprint/Player/Struct/ST_Weapon` (`/Game/Bluprint/Player/Struct/F_Weapon.F_WeaponInfo` (`/Game/Bluprint/Weapons/BP_WeaponBase.Name` (stale `SRV_Fire` Weapon)))))
  (`self.MC_VFXShoot` _muzzleflash (`/Game/Bluprint/Weapons/BP_WeaponBase.Weapon` (stale `SRV_Fire` Weapon)) _soundsfx (`self.K2_GetActorLocation`) :!label _label_6)
  (bind (_outhit _returnvalue) (`KismetSystemLibrary.LineTraceSingle` :`Start` (stale `SRV_Fire` Start) :`End` (stale `SRV_Fire` End) :`TraceChannel` "TraceTypeQuery1" :`DrawDebugType` "Persistent"))
  (if _returnvalue
    (bind (_bblockinghit _binitialoverlap _time _distance _location _impactpoint _normal _impactnormal _physmat _hitactor) (`GameplayStatics.BreakHitResult` _outhit))
    (if (and _bblockinghit (`self.ActorHasTag` _hitactor "player"))
      (`KismetSystemLibrary.PrintString` "Hello"))))

(event `ShootWeaponLoop`
  (goto _label_6))

(event `MC_VFXShoot`
  (params (VFX :type "ParticleSystem Object Reference") (Weapon :type "SceneComponent Object Reference") (Sound :type "SoundBase Object Reference") (Location :type "Vector Structure"))
  (`GameplayStatics.SpawnEmitterAttached` VFX Weapon "VFXShoot")
  (`GameplayStatics.SpawnSoundAtLocation` Sound Location (struct) 1.0 1.0 0.0 null null))

(event `SetsEquipWeapon`
  (params (bIsEqipWeapon :type Boolean))
  (`self.SRV_SetsEquipWeapon` bIsEqipWeapon))

(event `SRV_SetsEquipWeapon`
  (params (bIsEqipWeapon :type Boolean))
  (bind _output_get (set `self.bIsEqipWeapon` bIsEqipWeapon))
  (if _output_get
    (`self.MC_EquipWeapon` "NewEnumerator1")))

(fn `F_Crouch`
  (params (crouch :type Boolean))
  (locals (NewLocalVar :type Boolean))
  (bind _output_get (set `local.NewLocalVar` crouch))
  (`/Engine/EditorBlueprintResources/ActorMacros.Switch Has Authority`
    (:`Authority`
      _)
    (:`Remote`
      (`self.SRV_Crouch` _output_get)))
  (if (`local.NewLocalVar`)
    (`self.Crouch`)
    (set `self.bCrouch` true)
    (else
      (`self.UnCrouch`)
      (set `self.bCrouch` false))))

(fn `f_jump`
  (returns (ReturnValue :type Boolean))
  (return (not (`NavMovementComponent.IsFalling` (`self.CharacterMovement`)))))

(fn `F_Walk`
  (params (state :type Boolean))
  (locals (WalkLocal :type Boolean))
  (bind _output_get (set `local.WalkLocal` state))
  (`/Engine/EditorBlueprintResources/ActorMacros.Switch Has Authority`
    (:`Authority`
      _)
    (:`Remote`
      (`self.SRV_WAlk` _output_get)))
  (if (`local.WalkLocal`)
    (set `CharacterMovementComponent.MaxWalkSpeed` (`self.Max Walk Speed`) (`self.CharacterMovement`))
    (set `self.bWalk` true)
    (else
      (set `CharacterMovementComponent.MaxWalkSpeed` (`self.Run Speed`) (`self.CharacterMovement`))
      (set `self.bWalk` false))))

(fn `GetpalyerRef`
  (returns (Player :type "/Game/Bluprint/Player/BP_PlayerBase Object Reference"))
  (return self))

(fn `LineTraseShoot`
  (returns (ReturnValue :type "Vector Structure") (ReturnValue2 :type "Vector Structure"))
  (bind _playercontroller (message `/Game/Bluprint/Player/interface/INT_PlayerController.Get Controller Player ref` (`self.GetController`)))
  (bind _playercameramanager (`PlayerController.PlayerCameraManager` _playercontroller))
  (bind _returnvalue (`PlayerCameraManager.GetCameraLocation` _playercameramanager))
  (return _returnvalue (+ _returnvalue (* (`self.GetActorForwardVector` _playercameramanager) 20000))))

(fn `OnRep_dropweapon`
  (bind _weapon (`/Game/Bluprint/Weapons/BP_WeaponBase.Weapon` (`self.dropweapon`)))
  (bind _dropweapon (`self.dropweapon`)
    (:`then`
      (`self.K2_DetachFromActor` _dropweapon "KeepWorld" "KeepWorld" "KeepWorld")
      (`PrimitiveComponent.SetCollisionEnabled` _weapon "PhysicsOnly")
      (`PrimitiveComponent.SetSimulatePhysics` _weapon true)
      (`PrimitiveComponent.SetCollisionEnabled` (`/Game/Bluprint/Weapons/BP_WeaponBase.Sphere` (`self.dropweapon`)) "QueryOnly"))
    (:`else`)))

(fn `OnRep_Weapon`
  (bind _weapon (`self.Weapon`))
  (bind _weapon_2 (`/Game/Bluprint/Weapons/BP_WeaponBase.Weapon` _weapon))
  (bind _weapon_3 (`self.Weapon`)
    (:`then`
      (bind _weapon_4 (`/Game/Bluprint/Weapons/BP_WeaponBase.Weapon` _weapon_3))
      (`PrimitiveComponent.SetSimulatePhysics` _weapon_4 false)
      (`PrimitiveComponent.SetCollisionEnabled` _weapon_4 "NoCollision")
      (`PrimitiveComponent.SetCollisionEnabled` (`/Game/Bluprint/Weapons/BP_WeaponBase.Sphere` (`self.Weapon`)) "NoCollision")
      (`SceneComponent.K2_AttachToComponent` _weapon_2 (`/Game/Bluprint/Weapons/BP_WeaponBase.DefaultSceneRoot` _weapon) "None" "SnapToTarget" "SnapToTarget" "SnapToTarget" true)
      (`SceneComponent.ResetRelativeTransform` _weapon_2)
      (`self.K2_AttachToComponent` (`self.Weapon`) (`self.Mesh`) "S_Rifle" "SnapToTarget" "SnapToTarget" "SnapToTarget" true)
      (`self.SetEquipedWeapon` (`self.EqiupWeapon`)))
    (:`else`)))

(fn `UserConstructionScript`)